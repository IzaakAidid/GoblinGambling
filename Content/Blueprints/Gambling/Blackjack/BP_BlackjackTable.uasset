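; Blackjack table Blueprint for the gambling game that drives a bets-closing countdown display.
; On BeginPlay it hands the BP_BetsClosedTimer widget in its BetsClosingWidget component a short betting window and a reference to itself.
; The BetPlaced event makes that widget component visible and resets the timer, so each call restarts the countdown.
; No card dealing or game rules are implemented in these graphs.
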(event EventBeginPlay
  (bind _asbp_bets_closed_timer (Utilities|Casting|CastToBP_BetsClosedTimer (UserInterface|GetUserWidgetObject (Variables|Default|GetBetsClosingWidget))))
  (Variables|/Game/Blueprints/Gambling/Blackjack/BlackjackWidgets/BP_BetsClosedTimer.BP_BetsClosedTimer_C|SetBetsPlacedTime _asbp_bets_closed_timer 5.0)
  (Variables|/Game/Blueprints/Gambling/Blackjack/BlackjackWidgets/BP_BetsClosedTimer.BP_BetsClosedTimer_C|SetCardTable _asbp_bets_closed_timer self))

(event Collision|EventActorBeginOverlap
  (params (OtherActor :type Actor%20Object%20Reference)))

(event EventTick
  (params (DeltaSeconds :type Float%20%28single-precision%29)))

(event EventBetPlaced
  (bind _betsclosingwidget (Variables|Default|GetBetsClosingWidget))
  (Rendering|SetVisibility _betsclosingwidget true false)
  (bind _asbp_bets_closed_timer (Utilities|Casting|CastToBP_BetsClosedTimer (UserInterface|GetUserWidgetObject _betsclosingwidget)))
  (Default|Reset _asbp_bets_closed_timer))

(fn ConstructionScript)